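; Voice assistant actor that listens while something overlaps its Activator and answers aloud with lip sync, using the HMI processors.
; BeginPlay creates a chain of Whisper speech-to-text, Llama chat, Piper text-to-speech and OVR lip sync from named model files.
; Each captured sentence interrupts current output, then gets transcribed and prompted; streamed reply batches are voiced, lip-synced and played as they arrive.
; Leaving the overlap stops capture, cancels pending work and stops the chain.
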(event OnSentenceCaptured(HMIVoiceCapture)
  (params (Wave :type HMI%20Wave%20Handle%20Structure))
  (CallFunction|Interrupt)
  (bind _result (|STTAsync (Variables|Default|GetProcSTT) "None" Wave "en")
    (:Complete
      (bind _batchtext (|PromptAsync (Variables|Default|GetProcChat) "None" (.text _result) (Utilities|Array|MakeArray (Utilities|Struct|MakeHMIChatMessage "system" "You are a helpful assistant. Convert the output text into a format suitable for text-to-speech. Ensure that numbers, symbols, and abbreviations are expanded for clarity when read aloud. Expand all abbreviations to their full spoken forms.")) 0 0 1.0 1.0 true)
        (:Progress
          (bind _result_2 (|TTSAsync (Variables|Default|GetProcTTS) "None" _batchtext "0" 1.0)
            (:Complete
              (bind (_input _result_3) (|LipSyncAsync (Variables|Default|GetProcLipSync) "None" (.wave _result_2))
                (:Complete
                  (Class|HMIWavePlayerComponent|Play (Variables|Default|GetHMIWavePlayer) "None" (.wave _input) (.sequence _result_3)))))))))))

(event OnComponentBeginOverlap(Activator)
  (params (OverlappedComponent :type Primitive%20Component%20Object%20Reference) (OtherActor :type Actor%20Object%20Reference) (OtherComp :type Primitive%20Component%20Object%20Reference) (OtherBodyIndex :type Integer) (bFromSweep :type Boolean) (SweepResult :type Hit%20Result%20Structure%20%28by%20ref%29))
  (Class|HMIVoiceCaptureComponent|StartCapture (Variables|Default|GetHMIVoiceCapture))
  (Class|HMISubsystemStatics|StartChain (Variables|Default|GetProcChain)))

(event OnComponentEndOverlap(Activator)
  (params (OverlappedComponent :type Primitive%20Component%20Object%20Reference) (OtherActor :type Actor%20Object%20Reference) (OtherComp :type Primitive%20Component%20Object%20Reference) (OtherBodyIndex :type Integer))
  (Class|HMIVoiceCaptureComponent|StopCapture (Variables|Default|GetHMIVoiceCapture))
  (CallFunction|Interrupt)
  (Class|HMISubsystemStatics|StopChain (Variables|Default|GetProcChain) false))

(event Custom|Interrupt
  (Class|HMISubsystemStatics|CancelChain (Variables|Default|GetProcChain) true)
  (Class|HMIWavePlayerComponent|Stop (Variables|Default|GetHMIWavePlayer) true)
  (Class|HMILipSyncComponent|ResetLipSync (Variables|Default|GetHMILipSync)))

(event EventBeginPlay
  (bind _returnvalue (Class|HMISpeechtoTextWhisper|GetorCreateSTTWhisper "None" "ggml-small-q8_0.bin" true 4 "" false))
  (Variables|Default|SetProcSTT _returnvalue)
  (bind _returnvalue_2 (Class|HMITexttoSpeechPiper|GetorCreateTTSPiper "None" "en_US-libritts_r-medium.onnx" false "" 1.0))
  (Variables|Default|SetProcTTS _returnvalue_2)
  (bind _returnvalue_3 (Class|HMIChatLlama|GetorCreateChatLlama "None" "Llama-3.2_1b_Uncensored_RP_Aesir.gguf" 0 4))
  (Variables|Default|SetProcChat _returnvalue_3)
  (bind _returnvalue_4 (Class|HMILipSyncOVR|GetorCreateLipSyncOVR "None" "ovrlipsync_offline_model.pb" false))
  (Variables|Default|SetProcLipSync _returnvalue_4)
  (Variables|Default|SetProcChain (Utilities|Array|MakeArray (Variables|Default|GetProcSTT) (Variables|Default|GetProcChat) (Variables|Default|GetProcTTS) (Variables|Default|GetProcLipSync))))

(fn ConstructionScript)